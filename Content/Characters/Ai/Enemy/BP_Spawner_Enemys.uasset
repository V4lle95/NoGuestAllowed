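; Enemy spawner actor that stays idle until SpawnSecondPhase is called, then spawns a limited number of enemies.
; A repeating timer calls SpawnEnemy, which only acts while Looping is set and waits TimeBeforeSpawning before each spawn.
; Spawn positions are random points within a box sized in the construction script, offset from the actor's location.
; The spawner destroys itself upon reaching MaxNumberOfEnemys.
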(event `Spawn Enemy`
  (bind _box (`self.Box`))
  (if (`self.Looping`)
    (`KismetSystemLibrary.Delay` (`self.Time Before Spawning`))
    (`|SpawnActorFromClass` (`self.EnemysActors`) (`KismetMathLibrary.MakeTransform` (+ (+ (`self.K2_GetActorLocation`) (`self.GetActorForwardVector`)) (`KismetMathLibrary.RandomPointInBoundingBox` (`SceneComponent.RelativeLocation` _box) (`BoxComponent.BoxExtent` _box)))) "Undefined" "OverrideRootScale" null null)
    (bind _output_get (set `self.number of enemys` (+ (`self.number of enemys`) 1.0)))
    (if (== (`self.Max number of enemys`) _output_get)
      (set `self.Looping` false)
      (`self.K2_DestroyActor`)
      (else
        (set `self.Looping` true)))))

(event `self.ReceiveBeginPlay`
  (set `self.Looping` false)
  (`KismetSystemLibrary.K2_SetTimerDelegate` (delegate `Spawn Enemy`) 3.0 true))

(event `/Game/Characters/Player/Game_BPI.Spawn Second Phase`
  (set `self.Looping` true))

(fn `UserConstructionScript`
  (`BoxComponent.SetBoxExtent` (`self.Box`) (`self.Box Extent Vec`) true))