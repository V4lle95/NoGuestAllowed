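; Master Blueprint for a player-interactable loot chest that grants a random data table item to the inventory.
; A looping timer replaces Tick, switching between distance waypoint and interact prompt while IsDone is true, and destroying the waypoint otherwise.
; Box overlap toggles input and custom-depth highlight.
; Interact plays a lid timeline whose finish attempts the item transfer, clearing IsDone on success.
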(event `self.ReceiveBeginPlay`
  (bind _aswaypoints (cast `/Game/Characters/Player/Phase_1/Waypoints/Waypoints` (`WidgetComponent.GetUserWidgetObject` (`self.Waypoint`))))
  (set `self.Waypoint Ref` _aswaypoints)
  (bind _asw_interact (cast `/Game/Characters/Player/Phase_1/Inventory/UI/W_Interact` (`WidgetComponent.GetUserWidgetObject` (`self.Interact Widget`))))
  (set `self.Interactive Ref` _asw_interact)
  (`KismetSystemLibrary.K2_SetTimerDelegate` (delegate `Fake Tick`) 0.05 true)
  (set `/Game/Characters/Player/Phase_1/Inventory/UI/W_Interact.Name` "Chest" (`self.Interactive Ref`))
  (set `/Game/Characters/Player/Phase_1/Waypoints/Waypoints.Image` "/Game/UI/UserUI/chest.chest" (`self.Waypoint Ref`)))

(event `Fake Tick`
  (bind _waypoint (`self.Waypoint`))
  (bind _waypoint_ref (`self.Waypoint Ref`))
  (if (`self.Is Done?`)
    (bind _distance (`/Game/Characters/Player/Phase_1/Waypoints/Waypoints.Distance To Actor` (`self.Waypoint Ref`) (`GameplayStatics.GetPlayerCharacter` 0) self))
    (if (<= _distance (`self.Render Distace`))
      (`/Game/Characters/Player/Phase_1/Waypoints/Waypoints.Deactivate` (`self.Waypoint Ref`))
      (`/Game/Characters/Player/Phase_1/Inventory/UI/W_Interact.Active` (`self.Interactive Ref`))
      (else
        (`/Game/Characters/Player/Phase_1/Waypoints/Waypoints.Update` _waypoint_ref _distance)
        (`/Game/Characters/Player/Phase_1/Waypoints/Waypoints.Activate` _waypoint_ref)
        (`/Game/Characters/Player/Phase_1/Inventory/UI/W_Interact.Deactivate` (`self.Interactive Ref`))))
    (else
      (`/Engine/EditorBlueprintResources/StandardMacros.IsValid` _waypoint
        (:`Is Valid`
          (`ActorComponent.K2_DestroyComponent` _waypoint))))))

(event `self.Box.OnComponentBeginOverlap`
  (params (OverlappedComponent :type "PrimitiveComponent Object Reference") (OtherActor :type "Actor Object Reference") (OtherComp :type "PrimitiveComponent Object Reference") (OtherBodyIndex :type Integer) (bFromSweep :type Boolean) (SweepResult :type "HitResult Structure (by ref)"))
  (if (== OtherActor (`GameplayStatics.GetPlayerPawn` 0))
    (`self.EnableInput` (`GameplayStatics.GetPlayerController` 0))
    (if (`self.Is Done?`)
      (`PrimitiveComponent.SetRenderCustomDepth` (`self.StaticMesh`) true)
      (`PrimitiveComponent.SetRenderCustomDepth` (`self.Top`) true)
      (else
        (`PrimitiveComponent.SetRenderCustomDepth` (`self.StaticMesh`) false)
        (`PrimitiveComponent.SetRenderCustomDepth` (`self.Top`) false)))))

(event `InputAction|interact`
  (params (Key :type "Key Structure"))
  (:`Pressed`
    (`/Engine/EditorBlueprintResources/StandardMacros.IsValid` (`GameplayStatics.GetPlayerCharacter` 0)
      (:`Is Valid`
        (if (not (`self.Chest Open?`))
          (set `self.Chest Open?` true)
          (`TimelineComponent.Stop` (`self.Chest`))
          (bind (_direction _alpha) (`Timeline|Chest` :!via `PlayFromStart`)
            (:`Update`
              (`SceneComponent.K2_SetRelativeRotation` (`self.Top`) (`KismetMathLibrary.RLerp` (struct) (struct :`Pitch` 45.0) _alpha) false false))
            (:`Finished`
              (`self.Add Random Stuff to Player`)
              (set `self.Chest Open?` false))))))))

(event `self.Box.OnComponentEndOverlap`
  (params (OverlappedComponent :type "PrimitiveComponent Object Reference") (OtherActor :type "Actor Object Reference") (OtherComp :type "PrimitiveComponent Object Reference") (OtherBodyIndex :type Integer))
  (bind _returnvalue (`GameplayStatics.GetPlayerController` 0))
  (if (== OtherActor (`GameplayStatics.GetPlayerPawn` 0))
    (`self.DisableInput` _returnvalue _returnvalue)
    (`self.EnableInput` (`GameplayStatics.GetPlayerPawn` 0) _returnvalue)
    (`PrimitiveComponent.SetRenderCustomDepth` (`self.StaticMesh`) false)
    (`PrimitiveComponent.SetRenderCustomDepth` (`self.Top`) false)
    (if (`self.Is Done?`)
      (`TimelineComponent.ReverseFromEnd` (`self.Chest`)))))

(fn `Add Random Stuff to Player`
  (bind _data_tabla (`self.Data Tabla`))
  (`/Engine/EditorBlueprintResources/StandardMacros.IsValid` _data_tabla
    (:`Is Valid`
      (bind _outrownames (`DataTableFunctionLibrary.GetDataTableRowNames` _data_tabla))
      (bind _returnvalue (`|GetDataTableRow` _data_tabla (`|GetArrayItem` _outrownames (`KismetMathLibrary.RandomIntegerInRange` 0 (`KismetArrayLibrary.Array_Length` _outrownames))))
        (:`then`
          (bind _asplayer_character (cast `/Game/Characters/Player/Phase_1/PlayerCharacter` (`GameplayStatics.GetPlayerPawn` 0)))
          (`/Engine/EditorBlueprintResources/StandardMacros.IsValid` _asplayer_character
            (:`Is Valid`
              (bind _added_ (`/Game/Characters/Player/Phase_1/PlayerCharacter.Item To Inventory` _asplayer_character _returnvalue))
              (if _added_
                (set `self.Is Done?` false)
                (else
                  (set `self.Is Done?` true))))))))))

(fn `UserConstructionScript`)