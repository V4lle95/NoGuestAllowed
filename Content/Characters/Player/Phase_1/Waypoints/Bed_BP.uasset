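; Bed objective in player phase one that starts the game's second phase when the player interacts with it.
; A looping timer swaps a distance waypoint for an interact widget within render range, while the trigger enables input and outlines the bed.
; Interacting once spawns an attached AI kid and notifies timer, spawners, traps, chest and UI.
; Non-player overlaps damage the kid reference cached at BeginPlay.
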(event `self.ReceiveBeginPlay`
  (bind _aswaypoints (cast `/Game/Characters/Player/Phase_1/Waypoints/Waypoints` (`WidgetComponent.GetUserWidgetObject` (`self.Waypoint`))))
  (set `self.Waypoint Ref` _aswaypoints)
  (bind _asw_interact (cast `/Game/Characters/Player/Phase_1/Inventory/UI/W_Interact` (`WidgetComponent.GetUserWidgetObject` (`self.Interactive Widget`))))
  (set `self.Interact Ref` _asw_interact)
  (`KismetSystemLibrary.K2_SetTimerDelegate` (delegate `Fake Tick`) 0.05 true)
  (set `/Game/Characters/Player/Phase_1/Inventory/UI/W_Interact.Name` "Start The Game \nBed" (`self.Interact Ref`))
  (bind _outactors (`GameplayStatics.GetAllActorsOfClass` "/Game/Characters/Ai/AI_Kid.AI_Kid_C"))
  (bind _output (`|GetArrayItem` _outactors))
  (`/Engine/EditorBlueprintResources/StandardMacros.IsValid` _output
    (:`Is Valid`
      (set `self.AI Kid` _output))))

(event `Fake Tick`
  (bind _waypoint_ref (`self.Waypoint Ref`))
  (if (`self.Waypoint?`)
    (bind _distance (`/Game/Characters/Player/Phase_1/Waypoints/Waypoints.Distance To Actor` (`self.Waypoint Ref`) (`GameplayStatics.GetPlayerCharacter` 0) self))
    (if (<= _distance (`self.Render Distance`))
      (`/Game/Characters/Player/Phase_1/Waypoints/Waypoints.Deactivate` (`self.Waypoint Ref`))
      (`/Game/Characters/Player/Phase_1/Inventory/UI/W_Interact.Active` (`self.Interact Ref`))
      (else
        (`/Game/Characters/Player/Phase_1/Waypoints/Waypoints.Update` _waypoint_ref _distance)
        (`/Game/Characters/Player/Phase_1/Waypoints/Waypoints.Activate` _waypoint_ref)
        (`/Game/Characters/Player/Phase_1/Inventory/UI/W_Interact.Deactivate` (`self.Interact Ref`))))))

(event `self.Trigger.OnComponentBeginOverlap`
  (params (OverlappedComponent :type "PrimitiveComponent Object Reference") (OtherActor :type "Actor Object Reference") (OtherComp :type "PrimitiveComponent Object Reference") (OtherBodyIndex :type Integer) (bFromSweep :type Boolean) (SweepResult :type "HitResult Structure (by ref)"))
  (bind _bed (`self.Bed`))
  (if (== OtherActor (`GameplayStatics.GetPlayerCharacter` 0))
    (`self.EnableInput` (`GameplayStatics.GetPlayerController` 0))
    (if (`self.Waypoint?`)
      (`PrimitiveComponent.SetRenderCustomDepth` _bed true)
      (else
        (`PrimitiveComponent.SetRenderCustomDepth` _bed false)))
    (else
      (`GameplayStatics.ApplyDamage` (`self.AI Kid`) 5.0 null self))))

(event `self.Trigger.OnComponentEndOverlap`
  (params (OverlappedComponent :type "PrimitiveComponent Object Reference") (OtherActor :type "Actor Object Reference") (OtherComp :type "PrimitiveComponent Object Reference") (OtherBodyIndex :type Integer))
  (bind _returnvalue (`GameplayStatics.GetPlayerController` 0))
  (if (== OtherActor (`GameplayStatics.GetPlayerCharacter` 0))
    (`self.EnableInput` (`GameplayStatics.GetPlayerCharacter` 0) _returnvalue)
    (`self.DisableInput` _returnvalue)
    (`PrimitiveComponent.SetRenderCustomDepth` (`self.Bed`) false)))

(event `InputAction|interact`
  (params (Key :type "Key Structure"))
  (bind _scene (`self.Scene`))
  (:`Pressed`
    (`/Engine/EditorBlueprintResources/StandardMacros.DoOnce` false
      (:`Completed`
        (`|ExecutionSequence`
          (:`then_0`
            (bind _outactors (`GameplayStatics.GetAllActorsOfClass` "/Game/Characters/Player/FakePlayerStart.FakePlayerStart_C"))
            (message `/Game/Characters/Player/Game_BPI.Spawn Second Phase` (`|GetArrayItem` _outactors)))
          (:`then_1`
            (bind _outactors_2 (`GameplayStatics.GetAllActorsOfClass` "/Game/Characters/Player/Phase_2/Timer.Timer_C"))
            (message `/Game/Characters/Player/Game_BPI.Spawn Second Phase` (`|GetArrayItem` _outactors_2)))
          (:`then_2`
            (bind _returnvalue (`|SpawnActorFromClass` "/Game/Characters/Ai/AI_Kid.AI_Kid_C" (`KismetMathLibrary.MakeTransform` (`SceneComponent.K2_GetComponentLocation` _scene) (`KismetMathLibrary.Conv_VectorToRotator` (`SceneComponent.GetForwardVector` _scene))) "Undefined" "OverrideRootScale" null 500.0 500.0 null null))
            (`self.K2_AttachToComponent` _returnvalue (`self.Scene`) "None" "SnapToTarget" "SnapToTarget" "KeepWorld" true))
          (:`then_3`
            (`/Game/Characters/Player/Phase_1/Waypoints/Waypoints.Deactivate` (`self.Waypoint Ref`))
            (`/Game/Characters/Player/Phase_1/Inventory/UI/W_Interact.Deactivate` (`self.Interact Ref`)))
          (:`then_4`
            (set `self.Waypoint?` false)
            (`PrimitiveComponent.SetRenderCustomDepth` (`self.Bed`) false))
          (:`then_5`
            (bind _outactors_3 (`GameplayStatics.GetAllActorsOfClass` "/Game/Characters/Player/Phase_1/Inventory/Chest/BP_Master_Chest.BP_Master_Chest_C"))
            (bind _output (`|GetArrayItem` _outactors_3))
            (`/Engine/EditorBlueprintResources/StandardMacros.IsValid` _output
              (:`Is Valid`
                (set `/Game/Characters/Player/Phase_1/Inventory/Chest/BP_Master_Chest.Is Done?` false _output)
                (`/Game/Characters/Player/Phase_1/Waypoints/Waypoints.Deactivate` (`/Game/Characters/Player/Phase_1/Inventory/Chest/BP_Master_Chest.Waypoint Ref` _output))
                (`/Game/Characters/Player/Phase_1/Inventory/UI/W_Interact.Deactivate` (`/Game/Characters/Player/Phase_1/Inventory/Chest/BP_Master_Chest.Interactive Ref` _output)))))
          (:`then_6`
            (`KismetSystemLibrary.Delay` 1.0)
            (bind _foundwidgets (`WidgetBlueprintLibrary.GetAllWidgetsOfClass` "/Game/UI/UserUI/Phase_2/User_UI.User_UI_C" false))
            (bind _output_2 (`|GetArrayItem` _foundwidgets))
            (`/Engine/EditorBlueprintResources/StandardMacros.IsValid` _output_2
              (:`Is Valid`
                (set `/Game/UI/UserUI/Phase_2/User_UI.Parachute?` true _output_2))))
          (:`then_7`
            (bind _outactors_4 (`GameplayStatics.GetAllActorsOfClass` "/Game/Characters/Ai/Enemy/BP_Spawner_Enemys.BP_Spawner_Enemys_C"))
            (for _array_element _outactors_4
              (`/Engine/EditorBlueprintResources/StandardMacros.IsValid` _array_element
                (:`Is Valid`
                  (message `/Game/Characters/Player/Game_BPI.Spawn Second Phase` _array_element)))))
          (:`then_8`
            (bind _outactors_5 (`GameplayStatics.GetAllActorsOfClass` "/Game/Props/Blueprints/Decoy_Trap_BP.Decoy_Trap_BP_C"))
            (message `/Game/Characters/Player/Game_BPI.Traps go online` _outactors_5)
            (bind _outactors_6 (`GameplayStatics.GetAllActorsOfClass` "/Game/Props/Blueprints/OutOfTheUserCameraLocation_BP.OutOfTheUserCameraLocation_BP_C"))
            (for _array_element_2 _outactors_6
              (`/Engine/EditorBlueprintResources/StandardMacros.IsValid` _array_element_2
                (:`Is Valid`
                  (set `/Game/Props/Blueprints/OutOfTheUserCameraLocation_BP.Second Phase?` true _array_element_2)
                  (`PrimitiveComponent.SetRenderCustomDepth` (`self.Bed`) true))))))))))

(fn `UserConstructionScript`)