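; Chest prop that destroys itself with an explosion effect once its Steal counter equals 1.
; A looping timer started on BeginPlay polls Steal, then a DoOnce gate triggers a one-second delay, the emitter spawn and the actor's destruction.
; Each AI_Guard that begins overlapping the Box component decrements Steal by one.
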(event `self.ReceiveBeginPlay`
  (`KismetSystemLibrary.K2_SetTimerDelegate` (delegate `Start`) 0.1 true))

(event `Start`
  (if (== (`self.Steal`) 1)
    (`/Engine/EditorBlueprintResources/StandardMacros.DoOnce` false
      (:`Completed`
        (`KismetSystemLibrary.Delay` 1.0)
        (`GameplayStatics.SpawnEmitterAtLocation` "/Game/StarterContent/Particles/P_Explosion.P_Explosion" (`self.K2_GetActorLocation`))
        (`self.K2_DestroyActor`)))))

(event `self.Box.OnComponentBeginOverlap`
  (params (OverlappedComponent :type "PrimitiveComponent Object Reference") (OtherActor :type "Actor Object Reference") (OtherComp :type "PrimitiveComponent Object Reference") (OtherBodyIndex :type Integer) (bFromSweep :type Boolean) (SweepResult :type "HitResult Structure (by ref)"))
  (bind _asai_guard (cast `/Game/Characters/Ai/Enemy/AI_Guard` OtherActor))
  (`/Engine/EditorBlueprintResources/StandardMacros.IsValid` _asai_guard
    (:`Is Valid`
      (set `self.Steal` (- (`self.Steal`) 1)))))

(fn `UserConstructionScript`)