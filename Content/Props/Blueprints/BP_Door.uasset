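; BP_Door is a door prop that swings open when an actor enters its Trigger and closes when an overlap ends.
; The actor's position in the door's local space picks the yaw direction of the quarter-turn swing.
; Separate SwingOpen and SwingClose timelines stop each other and lerp from the door's current rotation, so interrupted swings continue smoothly.
; Overlaps are neither filtered nor counted.
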(event `self.Trigger.OnComponentBeginOverlap`
  (params (OverlappedComponent :type "PrimitiveComponent Object Reference") (OtherActor :type "Actor Object Reference") (OtherComp :type "PrimitiveComponent Object Reference") (OtherBodyIndex :type Integer) (bFromSweep :type Boolean) (SweepResult :type "HitResult Structure (by ref)"))
  (bind _door (`self.Door`))
  (bind _returnvalue_x (`KismetMathLibrary.BreakVector` (`KismetMathLibrary.LessLess_VectorRotator` (- (`self.K2_GetActorLocation`) (`self.K2_GetActorLocation` OtherActor)) (`self.K2_GetActorRotation`))))
  (`TimelineComponent.Stop` (`self.Swing Close`))
  (set `self.Open Direnction` (> _returnvalue_x 0.0))
  (bind (_direction _rotation) (`Timeline|Swing Open` :!via `PlayFromStart`)
    (:`Update`
      (`SceneComponent.K2_SetRelativeRotation` _door (`KismetMathLibrary.RLerp` (`SceneComponent.RelativeRotation` _door) (`KismetMathLibrary.MakeRotator` 0.0 0.0 (select `bool` (`self.Open Direnction`) :`false` 90.0 :`true` -90.0 :!type "Float (single-precision)")) _rotation true) false false))))

(event `self.Trigger.OnComponentEndOverlap`
  (params (OverlappedComponent :type "PrimitiveComponent Object Reference") (OtherActor :type "Actor Object Reference") (OtherComp :type "PrimitiveComponent Object Reference") (OtherBodyIndex :type Integer))
  (bind _door (`self.Door`))
  (`TimelineComponent.Stop` (`self.Swing Open`))
  (bind (_direction _rotation) (`Timeline|Swing Close` :!via `PlayFromStart`)
    (:`Update`
      (`SceneComponent.K2_SetRelativeRotation` _door (`KismetMathLibrary.RLerp` (`SceneComponent.RelativeRotation` _door) (struct) _rotation true) false false))))

(fn `UserConstructionScript`)