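; Elevator prop that carries a static mesh along a spline, driven by a timeline that plays forward or reverses based on an IsBottom flag.
; Outside Phase2, overlapping the box enables the interact input and shows a prompt widget, and leaving during an upward run reverses it.
; In Phase2, clicking the box triggers it and cursor hover toggles custom depth; TrapsGoOnline hides the widget.
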(event `self.ReceiveBeginPlay`
  (bind (_returnvalue_roll _returnvalue_pitch _returnvalue_yaw) (`KismetMathLibrary.BreakRotator` (`SplineComponent.GetRotationAtDistanceAlongSpline` (`self.Spline`) 0.0 "Local")))
  (`SceneComponent.K2_SetRelativeRotation` (`self.StaticMesh`) (`KismetMathLibrary.MakeRotator` _returnvalue_roll 0.0 _returnvalue_yaw) false false)
  (bind _asiteract_w (cast `/Game/Characters/Player/Phase_1/Waypoints/Iteract_w` (`WidgetComponent.GetUserWidgetObject` (`self.Widget`))))
  (set `self.Widget Iteract` _asiteract_w))

(event `self.Box.OnClicked`
  (params (TouchedComponent :type "PrimitiveComponent Object Reference") (ButtonPressed :type "Key Structure"))
  (if (`self.Phase 2?`)
    (if (`self.Is Bottom?`) :!label _label
      (bind (_direction _move) (`Timeline|Move Platform` :!label _label_2)
        (:`Update`
          (if (`self.Is Bottom?`)
            (set `self.Progress?` true))
          (bind _returnvalue (* _move (`SplineComponent.GetSplineLength` (`self.Spline`))))
          (`SceneComponent.K2_SetWorldLocation` (`self.StaticMesh`) (`SplineComponent.GetLocationAtDistanceAlongSpline` (`self.Spline`) _returnvalue "World") false false)
          (bind (_returnvalue_roll _returnvalue_pitch _returnvalue_yaw) (`KismetMathLibrary.BreakRotator` (`SplineComponent.GetRotationAtDistanceAlongSpline` (`self.Spline`) _returnvalue "Local")))
          (`SceneComponent.K2_SetRelativeRotation` (`self.StaticMesh`) (`KismetMathLibrary.MakeRotator` _returnvalue_roll 0.0 _returnvalue_yaw) false false))
        (:`Finished`
          (if (`self.Is Bottom?`)
            (set `self.Is Bottom?` false)
            (set `self.Progress?` false)
            (else
              (set `self.Is Bottom?` true)))))
      (else
        (goto _label_2 :!via `Reverse`)))))

(event `InputAction|interact`
  (params (Key :type "Key Structure"))
  (:`Pressed`
    (goto _label)))

(event `self.Box.OnComponentBeginOverlap`
  (params (OverlappedComponent :type "PrimitiveComponent Object Reference") (OtherActor :type "Actor Object Reference") (OtherComp :type "PrimitiveComponent Object Reference") (OtherBodyIndex :type Integer) (bFromSweep :type Boolean) (SweepResult :type "HitResult Structure (by ref)"))
  (if (and (== OtherActor (`GameplayStatics.GetPlayerPawn` 0)) (not (`self.Phase 2?`)))
    (`self.EnableInput` (`GameplayStatics.GetPlayerController` 0))
    (`/Game/Characters/Player/Phase_1/Waypoints/Iteract_w.Visible ` (`self.Widget Iteract`))))

(event `self.Box.OnComponentEndOverlap`
  (params (OverlappedComponent :type "PrimitiveComponent Object Reference") (OtherActor :type "Actor Object Reference") (OtherComp :type "PrimitiveComponent Object Reference") (OtherBodyIndex :type Integer))
  (bind _returnvalue (`GameplayStatics.GetPlayerController` 0))
  (if (and (== OtherActor (`GameplayStatics.GetPlayerPawn` 0)) (not (`self.Phase 2?`)))
    (if (`self.Progress?`)
      (`TimelineComponent.Reverse` (`self.Move Platform`))
      (set `self.Is Bottom?` false))
    (`self.EnableInput` (`GameplayStatics.GetPlayerCharacter` 0) _returnvalue)
    (`self.DisableInput` _returnvalue)
    (`/Game/Characters/Player/Phase_1/Waypoints/Iteract_w.Not Visible` (`self.Widget Iteract`))))

(event `self.ReceiveActorBeginCursorOver`
  (if (`self.Phase 2?`)
    (`PrimitiveComponent.SetRenderCustomDepth` (`self.StaticMesh`) true)))

(event `self.ReceiveActorEndCursorOver`
  (if (`self.Phase 2?`)
    (`PrimitiveComponent.SetRenderCustomDepth` (`self.StaticMesh`) false)))

(event `/Game/Characters/Player/Game_BPI.Traps go online`
  (`/Game/Characters/Player/Phase_1/Waypoints/Iteract_w.All not Visible` (`self.Widget Iteract`)))

(fn `UserConstructionScript`)