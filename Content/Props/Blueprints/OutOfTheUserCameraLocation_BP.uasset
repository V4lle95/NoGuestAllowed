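; Out-of-range trigger volume that shows the OutofRangeUI screen when the player enters it, or when an AI_Kid enters during SecondPhase.
; Player overlap disables input, then shares the AI path: remove the player HUD widgets and play the Transition timeline.
; The timeline animates a Material Parameter Collection scalar for the screen transition, then creates the out-of-range widget.
; The construction script scales the Cube to the collision component's world scale.
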(event `self.ReceiveActorBeginOverlap`
  (params (OtherActor :type "Actor Object Reference"))
  (if (`self.Second Phase?`)
    (`TimelineComponent.Stop` (`self.Transition`))
    (bind _outactors (`GameplayStatics.GetAllActorsOfClass` "/Game/Characters/Ai/AI_Kid.AI_Kid_C"))
    (for _array_element _outactors
      (if (== _array_element OtherActor)
        (`self.Remove Widgets` :!label _label)
        (bind (_direction _alpha) (`Timeline|Transition` :!via `PlayFromStart`)
          (:`Update`
            (`KismetMaterialLibrary.SetScalarParameterValue` "/Game/Materials/PostProcess/Transition/Transition.Transition" "Ammount UP" (`KismetMathLibrary.Lerp` -1.0 1.0 _alpha)))
          (:`Finished`
            (bind _returnvalue (`|CreateWidget` "/Game/UI/UserUI/OutofRangeUI.OutofRangeUI_C"))
            (`UserWidget.AddToViewport` _returnvalue 0)))))))

(event `self.CollisionComponent.OnComponentBeginOverlap`
  (params (OverlappedComponent :type "PrimitiveComponent Object Reference") (OtherActor :type "Actor Object Reference") (OtherComp :type "PrimitiveComponent Object Reference") (OtherBodyIndex :type Integer) (bFromSweep :type Boolean) (SweepResult :type "HitResult Structure (by ref)"))
  (if (== OtherActor (`GameplayStatics.GetPlayerPawn` 0))
    (`self.DisableInput` (`GameplayStatics.GetPlayerCharacter` 0) (`GameplayStatics.GetPlayerController` 0))
    (goto _label)))

(fn `Remove Widgets`
  (`|ExecutionSequence`
    (:`then_0`
      (bind _foundwidgets (`WidgetBlueprintLibrary.GetAllWidgetsOfClass` "/Game/UI/UserUI/Phase_2/User_UI.User_UI_C" false))
      (bind _output (`|GetArrayItem` _foundwidgets))
      (`/Engine/EditorBlueprintResources/StandardMacros.IsValid` _output
        (:`Is Valid`
          (`Widget.RemoveFromParent` _output))))
    (:`then_1`
      (bind _foundwidgets_2 (`WidgetBlueprintLibrary.GetAllWidgetsOfClass` "/Game/Characters/Player/Phase_1/Inventory/UI/w_Player_UI.w_Player_UI_C" false))
      (bind _output_2 (`|GetArrayItem` _foundwidgets_2))
      (`/Engine/EditorBlueprintResources/StandardMacros.IsValid` _output_2
        (:`Is Valid`
          (`Widget.RemoveFromParent` _output_2)))))
  (return))

(fn `UserConstructionScript`
  (`SceneComponent.SetWorldScale3D` (`self.Cube`) (`SceneComponent.K2_GetComponentScale` (`self.CollisionComponent`))))