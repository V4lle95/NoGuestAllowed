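; Clickable spike trap that the player toggles during Phase2 to damage AI guards.
; Clicking the floor box flip-flops two timelines that scale the spike's height and switch its hitbox collision on or off.
; Guards overlapping the hitbox take damage read from the SpikeTrap row of the traps data table.
; Hovering in Phase2 swaps the cursor and toggles custom depth on the spike for highlighting.
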(event `self.Floor Box.OnClicked`
  (params (TouchedComponent :type "PrimitiveComponent Object Reference") (ButtonPressed :type "Key Structure"))
  (if (`self.Phase 2?`)
    (`/Engine/EditorBlueprintResources/StandardMacros.FlipFlop`
      (:`A`
        (`SceneComponent.SetVisibility` (`self.Spike`) true false)
        (bind (_direction _alpha) (`Timeline|Make Bigger` :!via `PlayFromStart`)
          (:`Update`
            (`SceneComponent.SetRelativeScale3D` (`self.Spike`) (`KismetMathLibrary.MakeVector` 1.0 1.0 _alpha)))
          (:`Finished`
            _))
        (`PrimitiveComponent.SetCollisionEnabled` (`self.Spike Box`) "QueryAndPhysics"))
      (:`B`
        (bind (_direction_2 _alpha_2) (`Timeline|Make Smaller` :!via `PlayFromStart`)
          (:`Update`
            (`SceneComponent.SetRelativeScale3D` (`self.Spike`) (`KismetMathLibrary.MakeVector` 1.0 1.0 _alpha_2)))
          (:`Finished`
            _))
        (`PrimitiveComponent.SetCollisionEnabled` (`self.Spike Box`) "NoCollision")))))

(event `self.Spike Box.OnComponentBeginOverlap`
  (params (OverlappedComponent :type "PrimitiveComponent Object Reference") (OtherActor :type "Actor Object Reference") (OtherComp :type "PrimitiveComponent Object Reference") (OtherBodyIndex :type Integer) (bFromSweep :type Boolean) (SweepResult :type "HitResult Structure (by ref)"))
  (bind _outactors (`GameplayStatics.GetAllActorsOfClass` "/Game/Characters/Ai/Enemy/AI_Guard.AI_Guard_C"))
  (for _array_element _outactors
    (if (== _array_element OtherActor)
      (bind _returnvalue (`|GetDataTableRow` "/Game/Blueprints/Traps_DataTable.Traps_DataTable" "SpikeTrap")
        (:`then`
          (`GameplayStatics.ApplyDamage` OtherActor (`.Damage_6_666D396E4E7235FFCE84008E808C7946` (break `/Game/Blueprints/TrapsStruct` _returnvalue)) null self))))))

(event `self.ReceiveActorBeginCursorOver`
  (if (`self.Phase 2?`)
    (set `PlayerController.CurrentMouseCursor` "GrabHandClosed" (`GameplayStatics.GetPlayerController` 0))
    (`PrimitiveComponent.SetRenderCustomDepth` (`self.Spike`) true)))

(event `self.ReceiveActorEndCursorOver`
  (if (`self.Phase 2?`)
    (set `PlayerController.CurrentMouseCursor` "GrabHand" (`GameplayStatics.GetPlayerController` 0))
    (`PrimitiveComponent.SetRenderCustomDepth` (`self.Spike`) false)))

(event `self.ReceiveBeginPlay`
  (`PrimitiveComponent.SetCollisionEnabled` (`self.Spike Box`) "NoCollision")
  (`SceneComponent.SetRelativeScale3D` (`self.Spike`) (1.0 1.0 0.0)))

(fn `UserConstructionScript`)