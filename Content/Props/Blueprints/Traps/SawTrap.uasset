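; SawTrap is a trap prop with a spinning saw and a box trigger for damage.
; On BeginPlay it plays the Moving timeline once from the start, adding its value to the Saw's relative pitch on each update.
; Box overlaps by any actor other than the first player's pawn call ApplyDamage with the trap as causer, but no damaged actor is wired into that call.
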(event `self.ReceiveBeginPlay`
  (`/Engine/EditorBlueprintResources/StandardMacros.DoOnce` false
    (:`Completed`
      (`self.move`))))

(event `move`
  (bind (_direction _y) (`Timeline|Moving` :!via `PlayFromStart`)
    (:`Update`
      (`SceneComponent.K2_AddRelativeRotation` (`self.Saw`) (`KismetMathLibrary.MakeRotator` 0.0 _y) false false))))

(event `self.Box.OnComponentBeginOverlap`
  (params (OverlappedComponent :type "PrimitiveComponent Object Reference") (OtherActor :type "Actor Object Reference") (OtherComp :type "PrimitiveComponent Object Reference") (OtherBodyIndex :type Integer) (bFromSweep :type Boolean) (SweepResult :type "HitResult Structure (by ref)"))
  (if (!= OtherActor (`GameplayStatics.GetPlayerPawn` 0))
    (`GameplayStatics.ApplyDamage` null 100.0 null self)))

(fn `UserConstructionScript`)