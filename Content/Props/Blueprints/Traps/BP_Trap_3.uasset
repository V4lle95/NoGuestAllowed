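; BP_Trap_3 is a click-activated knight trap whose sword damages actors other than the player pawn.
; Clicking the knight's collider eases the sword to a new pose, then resets its rotation with a sweep after a delay, with a flag blocking retriggering meanwhile.
; Sword collider overlaps apply randomized damage whether or not a swing is active.
; Cursor hover toggles custom depth on the knight for highlighting.
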(event `self.KnightCol.OnClicked`
  (params (TouchedComponent :type "PrimitiveComponent Object Reference") (ButtonPressed :type "Key Structure" :default "AnyKey"))
  (bind _sword (`self.Sword`))
  (if (`self.Sword Down?`)
    (`KismetSystemLibrary.MoveComponentTo` _sword (-30.0 0.0 90.0) (struct :`Pitch` 90.0) true true)
    (set `self.Sword Down?` false)
    (`KismetSystemLibrary.Delay` 1.0)
    (`SceneComponent.K2_SetRelativeRotation` _sword (struct :`Yaw` 80.0) true false)
    (`KismetSystemLibrary.Delay` 0.5)
    (set `self.Sword Down?` true)))

(event `self.SwordCol.OnComponentBeginOverlap`
  (params (OverlappedComponent :type "PrimitiveComponent Object Reference") (OtherActor :type "Actor Object Reference") (OtherComp :type "PrimitiveComponent Object Reference") (OtherBodyIndex :type Integer) (bFromSweep :type Boolean) (SweepResult :type "HitResult Structure (by ref)"))
  (if (!= OtherActor (`GameplayStatics.GetPlayerPawn` 0))
    (`GameplayStatics.ApplyDamage` OtherActor (* (`KismetMathLibrary.RandomFloatInRange` 20.0 50.0) (`KismetMathLibrary.RandomFloat`)) null self)))

(event `self.ReceiveActorBeginCursorOver`
  (`PrimitiveComponent.SetRenderCustomDepth` (`self.Knight`) true))

(event `self.ReceiveActorEndCursorOver`
  (`PrimitiveComponent.SetRenderCustomDepth` (`self.Knight`) false))

(fn `UserConstructionScript`)