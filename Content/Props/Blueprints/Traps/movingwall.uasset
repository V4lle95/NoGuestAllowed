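; Clickable moving wall trap that becomes active in Phase2, when TrapsGoOnline switches the Cube's material and its Pawn response from Block to Overlap.
; A click runs a timeline that slides the Cube along local Y, with direction set by a boolean and re-triggering blocked while moving.
; Box1 collides only during movement, damaging overlapping actors using the Traps_DataTable value.
; In Phase2, hovering changes cursor, material and custom-depth highlight.
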(event `self.Cube.OnClicked`
  (params (TouchedComponent :type "PrimitiveComponent Object Reference") (ButtonPressed :type "Key Structure"))
  (bind _cube (`self.Cube`))
  (if (`self.Phase 2?`) :!label _label
    (if (not (`self.Is Moving?`))
      (set `self.Is Moving?` true)
      (`TimelineComponent.Stop` (`self.Boxmoving`))
      (`PrimitiveComponent.SetCollisionEnabled` (`self.Box1`) "QueryAndPhysics")
      (bind (_direction _boxmoving) (`Timeline|Boxmoving` :`NewTime` 0.5 :!via `PlayFromStart`)
        (:`Update`
          (if (`self.Positive or Negative Location`)
            (`SceneComponent.K2_SetRelativeLocation` _cube (`KismetMathLibrary.MakeVector` 0.0 _boxmoving) false false)
            (else
              (`SceneComponent.K2_SetRelativeLocation` _cube (`KismetMathLibrary.MakeVector` 0.0 (* _boxmoving -1.0)) false false))))
        (:`Finished`
          (`PrimitiveComponent.SetCollisionEnabled` (`self.Box1`) "NoCollision")
          (set `self.Is Moving?` false))))))

(event `self.ReceiveActorOnClicked`
  (params (ButtonPressed :type "Key Structure"))
  (goto _label))

(event `self.Box1.OnComponentBeginOverlap`
  (params (OverlappedComponent :type "PrimitiveComponent Object Reference") (OtherActor :type "Actor Object Reference") (OtherComp :type "PrimitiveComponent Object Reference") (OtherBodyIndex :type Integer) (bFromSweep :type Boolean) (SweepResult :type "HitResult Structure (by ref)"))
  (bind _returnvalue (`|GetDataTableRow` "/Game/Blueprints/Traps_DataTable.Traps_DataTable" "MovingWall")
    (:`then`
      (`GameplayStatics.ApplyDamage` OtherActor (`.Damage_6_666D396E4E7235FFCE84008E808C7946` (break `/Game/Blueprints/TrapsStruct` _returnvalue)) null self))))

(event `self.ReceiveActorBeginCursorOver`
  (if (`self.Phase 2?`)
    (set `PlayerController.CurrentMouseCursor` "GrabHandClosed" (`GameplayStatics.GetPlayerController` 0))
    (`PrimitiveComponent.SetRenderCustomDepth` (`self.Cube`) true)
    (`PrimitiveComponent.SetMaterial` (`self.Cube`) 0 "/Game/Materials/Mat_master_Wall.Mat_master_Wall")))

(event `self.ReceiveActorEndCursorOver`
  (if (`self.Phase 2?`)
    (set `PlayerController.CurrentMouseCursor` "GrabHand" (`GameplayStatics.GetPlayerController` 0))
    (`PrimitiveComponent.SetRenderCustomDepth` (`self.Cube`) false)
    (`PrimitiveComponent.SetMaterial` (`self.Cube`) 0 "/Game/Materials/Mat_master_Wall_H.Mat_master_Wall_H")))

(event `self.ReceiveBeginPlay`
  (`PrimitiveComponent.SetCollisionEnabled` (`self.Box1`) "NoCollision")
  (`PrimitiveComponent.SetMaterial` (`self.Cube`) 0 "/Game/Materials/Mat_master_Wall.Mat_master_Wall")
  (`PrimitiveComponent.SetCollisionResponseToChannel` (`self.Cube`) "ECC_Pawn" "ECR_Block"))

(event `/Game/Characters/Player/Game_BPI.Traps go online`
  (`PrimitiveComponent.SetMaterial` (`self.Cube`) 0 "/Game/Materials/Mat_master_Wall_H.Mat_master_Wall_H")
  (`PrimitiveComponent.SetCollisionResponseToChannel` (`self.Cube`) "ECC_Pawn" "ECR_Overlap")
  (set `self.Phase 2?` true))

(fn `UserConstructionScript`)