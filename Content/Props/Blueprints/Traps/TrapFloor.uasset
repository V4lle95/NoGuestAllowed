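; Clickable trap floor prop whose two halves swing open in opposite roll directions through a timeline, once per DoOnce.
; TrapsGoOnline sets Phase2 and swaps both meshes to the highlight material.
; While Open and Phase2 are true, hovering changes the cursor, material and custom-depth outline.
; Clicking checks neither flag; the timeline clears Open and the outline and resets the cursor.
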(event `self.ReceiveActorOnClicked`
  (params (ButtonPressed :type "Key Structure"))
  (`/Engine/EditorBlueprintResources/StandardMacros.DoOnce` false
    (:`Completed`
      (bind (_direction _floorfallpart1) (`Timeline|FloorFallPart1`)
        (:`Update`
          (`SceneComponent.K2_SetRelativeRotation` (`self.1`) (`KismetMathLibrary.MakeRotator` (* _floorfallpart1 -1.0)) false false)
          (`SceneComponent.K2_SetRelativeRotation` (`self.2`) (`KismetMathLibrary.MakeRotator` _floorfallpart1) false false)
          (set `self.Open?` false)
          (`PrimitiveComponent.SetRenderCustomDepth` (`self.StaticMesh`) false)
          (`PrimitiveComponent.SetRenderCustomDepth` (`self.StaticMesh1`) false)
          (set `PlayerController.CurrentMouseCursor` "GrabHand" (`GameplayStatics.GetPlayerController` 0)))))))

(event `self.ReceiveActorBeginCursorOver`
  (if (and (`self.Open?`) (`self.Phase 2?`))
    (set `PlayerController.CurrentMouseCursor` "GrabHandClosed" (`GameplayStatics.GetPlayerController` 0))
    (`PrimitiveComponent.SetRenderCustomDepth` (`self.StaticMesh`) true)
    (`PrimitiveComponent.SetRenderCustomDepth` (`self.StaticMesh1`) true)
    (`PrimitiveComponent.SetMaterial` (`self.StaticMesh`) 0 "/Game/Materials/Mat_master_Black.Mat_master_Black")
    (`PrimitiveComponent.SetMaterial` (`self.StaticMesh1`) 0 "/Game/Materials/Mat_master_Black.Mat_master_Black")))

(event `self.ReceiveActorEndCursorOver`
  (if (and (`self.Open?`) (`self.Phase 2?`))
    (set `PlayerController.CurrentMouseCursor` "GrabHand" (`GameplayStatics.GetPlayerController` 0))
    (`PrimitiveComponent.SetRenderCustomDepth` (`self.StaticMesh`) false)
    (`PrimitiveComponent.SetRenderCustomDepth` (`self.StaticMesh1`) false)
    (`PrimitiveComponent.SetMaterial` (`self.StaticMesh1`) 0 "/Game/Materials/Mat_master_Black_H.Mat_master_Black_H")
    (`PrimitiveComponent.SetMaterial` (`self.StaticMesh`) 0 "/Game/Materials/Mat_master_Black_H.Mat_master_Black_H")))

(event `self.ReceiveBeginPlay`
  (`PrimitiveComponent.SetMaterial` (`self.StaticMesh`) 0 "/Game/Materials/Mat_master_Black.Mat_master_Black")
  (`PrimitiveComponent.SetMaterial` (`self.StaticMesh1`) 0 "/Game/Materials/Mat_master_Black.Mat_master_Black"))

(event `/Game/Characters/Player/Game_BPI.Traps go online`
  (`PrimitiveComponent.SetMaterial` (`self.StaticMesh1`) 0 "/Game/Materials/Mat_master_Black_H.Mat_master_Black_H")
  (`PrimitiveComponent.SetMaterial` (`self.StaticMesh`) 0 "/Game/Materials/Mat_master_Black_H.Mat_master_Black_H")
  (set `self.Phase 2?` true))

(fn `UserConstructionScript`)