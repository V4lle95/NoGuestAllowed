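; Clickable horse prop trap that launches AI guards.
; Clicking HorseTrigger eases the Horse component up and then down with timed relative moves, using IsUP to ignore clicks during the cycle.
; Any AI_Guard that begins overlapping HorseCol is launched along Z by LaunchAI, independent of whether the horse is moving.
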(event `self.ReceiveBeginPlay`)

(event `self.HorseTrigger.OnClicked`
  (params (TouchedComponent :type "PrimitiveComponent Object Reference") (ButtonPressed :type "Key Structure"))
  (bind _horse (`self.Horse`))
  (if (not (`self.Is UP?`))
    (set `self.Is UP?` true)
    (`KismetSystemLibrary.MoveComponentTo` _horse (0.0 0.0 60.0) (struct) true true)
    (`KismetSystemLibrary.Delay` 0.5)
    (`KismetSystemLibrary.MoveComponentTo` _horse (0.0 0.0 -120.0) (struct) true true)
    (`KismetSystemLibrary.Delay` 0.5)
    (set `self.Is UP?` false)))

(event `self.HorseCol.OnComponentBeginOverlap`
  (params (OverlappedComponent :type "PrimitiveComponent Object Reference") (OtherActor :type "Actor Object Reference") (OtherComp :type "PrimitiveComponent Object Reference") (OtherBodyIndex :type Integer) (bFromSweep :type Boolean) (SweepResult :type "HitResult Structure (by ref)"))
  (bind _asai_guard (cast `/Game/Characters/Ai/Enemy/AI_Guard` OtherActor))
  (`Character.LaunchCharacter` _asai_guard (`KismetMathLibrary.MakeVector` 0.0 0.0 (`self.Launch AI`)) false false))

(fn `UserConstructionScript`)