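; Clickable toxic trap prop that the player can switch on and off once TrapsGoOnline enables its Phase2 state.
; Clicks on the cube flip-flop the particle effect and a looping timer that damages every valid actor tracked by the box overlap each second.
; In Phase2, cursor hover changes the mouse cursor, swaps the cube's material and toggles custom depth rendering.
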(event `self.ReceiveBeginPlay`
  (`SceneComponent.SetHiddenInGame` (`self.ParticleSystem`) true false)
  (`PrimitiveComponent.SetMaterial` (`self.Cube`) 0 "/Game/Materials/Mat_master_Concrete.Mat_master_Concrete"))

(event `self.Cube.OnClicked`
  (params (TouchedComponent :type "PrimitiveComponent Object Reference") (ButtonPressed :type "Key Structure"))
  (bind _particlesystem (`self.ParticleSystem`))
  (if (`self.Phase 2?`)
    (`/Engine/EditorBlueprintResources/StandardMacros.FlipFlop`
      (:`A`
        (`SceneComponent.SetHiddenInGame` _particlesystem false false)
        (bind _returnvalue (`KismetSystemLibrary.K2_SetTimerDelegate` (delegate `DMG`) 1.0 true))
        (set `self.DMG Event` _returnvalue))
      (:`B`
        (`SceneComponent.SetHiddenInGame` _particlesystem true false)
        (`KismetSystemLibrary.K2_ClearAndInvalidateTimerHandle` (`self.DMG Event`))))))

(event `DMG`
  (for _array_element (`self.Hit Array`)
    (`/Engine/EditorBlueprintResources/StandardMacros.IsValid` _array_element
      (:`Is Valid`
        (`GameplayStatics.ApplyDamage` _array_element 50.0 (`self.GetInstigatorController` self) self)))))

(event `self.ReceiveActorBeginCursorOver`
  (if (`self.Phase 2?`)
    (set `PlayerController.CurrentMouseCursor` "GrabHandClosed" (`GameplayStatics.GetPlayerController` 0))
    (`PrimitiveComponent.SetRenderCustomDepth` (`self.Cube`) true)
    (`PrimitiveComponent.SetMaterial` (`self.Cube`) 0 "/Game/Materials/Mat_master_Concrete.Mat_master_Concrete")))

(event `self.ReceiveActorEndCursorOver`
  (if (`self.Phase 2?`)
    (set `PlayerController.CurrentMouseCursor` "GrabHand" (`GameplayStatics.GetPlayerController` 0))
    (`PrimitiveComponent.SetRenderCustomDepth` (`self.Cube`) false)
    (`PrimitiveComponent.SetMaterial` (`self.Cube`) 0 "/Game/Materials/Mat_master_Concrete_H.Mat_master_Concrete_H")))

(event `self.Box.OnComponentBeginOverlap`
  (params (OverlappedComponent :type "PrimitiveComponent Object Reference") (OtherActor :type "Actor Object Reference") (OtherComp :type "PrimitiveComponent Object Reference") (OtherBodyIndex :type Integer) (bFromSweep :type Boolean) (SweepResult :type "HitResult Structure (by ref)"))
  (bind _output_get (set `self.Hit Actor` OtherActor))
  (`KismetArrayLibrary.Array_Add` (`self.Hit Array`) _output_get))

(event `self.Box.OnComponentEndOverlap`
  (params (OverlappedComponent :type "PrimitiveComponent Object Reference") (OtherActor :type "Actor Object Reference") (OtherComp :type "PrimitiveComponent Object Reference") (OtherBodyIndex :type Integer))
  (bind _output_get (set `self.Hit Actor` OtherActor))
  (`KismetArrayLibrary.Array_RemoveItem` (`self.Hit Array`) _output_get))

(event `/Game/Characters/Player/Game_BPI.Traps go online`
  (`PrimitiveComponent.SetMaterial` (`self.Cube`) 0 "/Game/Materials/Mat_master_Concrete_H.Mat_master_Concrete_H")
  (set `self.Phase 2?` true))

(fn `UserConstructionScript`
  (`parent.UserConstructionScript`))