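; Clickable chandelier trap that drops from its mount to damage whatever its box overlaps.
; Clicking plays the Fall timeline, lowering the mesh, enabling box collision and destroying the actor after a short delay.
; Box overlaps apply damage read from the "Chandalier" row of Traps_DataTable.
; Hover toggles the grab cursor and custom-depth rendering, while TrapsGoOnline swaps the mesh's materials.
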(event `self.ReceiveBeginPlay`
  (`PrimitiveComponent.SetSimulatePhysics` (`self.Chandelier`) false)
  (`PrimitiveComponent.SetCollisionEnabled` (`self.Box`) "NoCollision")
  (`self.Set Material` "/Game/Materials/Mat_master_Black.Mat_master_Black"))

(event `self.Chandelier.OnClicked`
  (params (TouchedComponent :type "PrimitiveComponent Object Reference") (ButtonPressed :type "Key Structure"))
  (bind (_direction _fall) (`Timeline|Fall` :!via `PlayFromStart` :!label _label)
    (:`Update`
      (`SceneComponent.K2_SetRelativeLocation` (`self.Chandelier`) (`KismetMathLibrary.VLerp` (0.0 0.0 0.0) (0.0 0.0 -500.0) _fall) false false)
      (`PrimitiveComponent.SetCollisionEnabled` (`self.Box`) "QueryAndPhysics")
      (`KismetSystemLibrary.Delay` 2.0)
      (`self.K2_DestroyActor`))))

(event `self.ReceiveActorOnClicked`
  (params (ButtonPressed :type "Key Structure"))
  (goto _label :!via `PlayFromStart`))

(event `self.Box.OnComponentBeginOverlap`
  (params (OverlappedComponent :type "PrimitiveComponent Object Reference") (OtherActor :type "Actor Object Reference") (OtherComp :type "PrimitiveComponent Object Reference") (OtherBodyIndex :type Integer) (bFromSweep :type Boolean) (SweepResult :type "HitResult Structure (by ref)"))
  (bind _returnvalue (`|GetDataTableRow` "/Game/Blueprints/Traps_DataTable.Traps_DataTable" "Chandalier")
    (:`then`
      (`GameplayStatics.ApplyDamage` OtherActor (`.Damage_6_666D396E4E7235FFCE84008E808C7946` (break `/Game/Blueprints/TrapsStruct` _returnvalue)) null self))))

(event `/Game/Characters/Player/Game_BPI.Traps go online`
  (`self.Set Material` "/Game/Materials/Mat_master_Black_H.Mat_master_Black_H"))

(event `self.ReceiveActorBeginCursorOver`
  (set `PlayerController.CurrentMouseCursor` "GrabHandClosed" (`GameplayStatics.GetPlayerController` 0))
  (`PrimitiveComponent.SetRenderCustomDepth` (`self.Chandelier`) true))

(event `self.ReceiveActorEndCursorOver`
  (set `PlayerController.CurrentMouseCursor` "GrabHand" (`GameplayStatics.GetPlayerController` 0))
  (`PrimitiveComponent.SetRenderCustomDepth` (`self.Chandelier`) false))

(fn `Set Material`
  (params (Material :type "MaterialInterface Object Reference"))
  (bind _chandelier (`self.Chandelier`))
  (`PrimitiveComponent.SetMaterial` _chandelier 0 Material)
  (`PrimitiveComponent.SetMaterial` _chandelier 2 Material)
  (`PrimitiveComponent.SetMaterial` _chandelier 3 Material)
  (`PrimitiveComponent.SetMaterial` _chandelier 3 Material)
  (`PrimitiveComponent.SetMaterial` _chandelier 5 Material)
  (`PrimitiveComponent.SetMaterial` _chandelier 6 Material)
  (`PrimitiveComponent.SetMaterial` _chandelier 7 Material)
  (`PrimitiveComponent.SetMaterial` _chandelier 8 Material))

(fn `UserConstructionScript`)