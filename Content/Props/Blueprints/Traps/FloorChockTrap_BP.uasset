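; Floor electric trap that the player clicks to switch on and off once TrapsGoOnline starts Phase2.
; Each click flip-flops the Box's Pawn collision between Overlap and Ignore and shows or hides the arc particles.
; Overlapping actors are stored in EnemyArray and take fixed damage when they leave the Box, not on entry.
; In Phase2, hovering changes the cursor, swaps materials and toggles custom-depth rendering on both cubes.
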(event `self.ReceiveBeginPlay`
  (`SceneComponent.SetVisibility` (`self.ParticleSystem1`) false false)
  (`SceneComponent.SetVisibility` (`self.P_electricity_arc`) false false)
  (`SceneComponent.SetVisibility` (`self.ParticleSystem`) false false)
  (`PrimitiveComponent.SetCollisionResponseToChannel` (`self.Box`) "ECC_Pawn" "ECR_Ignore")
  (`PrimitiveComponent.SetMaterial` (`self.Cube1`) 0 "/Game/Materials/Mat_master_Black.Mat_master_Black")
  (`PrimitiveComponent.SetMaterial` (`self.Cube`) 0 "/Game/Materials/Mat_master_Black.Mat_master_Black"))

(event `self.Box.OnClicked`
  (params (TouchedComponent :type "PrimitiveComponent Object Reference") (ButtonPressed :type "Key Structure"))
  (if (`self.Phase 2?`)
    (`/Engine/EditorBlueprintResources/StandardMacros.FlipFlop`
      (:`A`
        (`PrimitiveComponent.SetCollisionResponseToChannel` (`self.Box`) "ECC_Pawn" "ECR_Overlap")
        (`SceneComponent.SetVisibility` (`self.ParticleSystem1`) true false)
        (`SceneComponent.SetVisibility` (`self.P_electricity_arc`) true false)
        (`SceneComponent.SetVisibility` (`self.ParticleSystem`) true false))
      (:`B`
        (`PrimitiveComponent.SetCollisionResponseToChannel` (`self.Box`) "ECC_Pawn" "ECR_Ignore")
        (`SceneComponent.SetVisibility` (`self.ParticleSystem1`) false false)
        (`SceneComponent.SetVisibility` (`self.P_electricity_arc`) false false)
        (`SceneComponent.SetVisibility` (`self.ParticleSystem`) false false)))))

(event `self.Box.OnComponentBeginOverlap`
  (params (OverlappedComponent :type "PrimitiveComponent Object Reference") (OtherActor :type "Actor Object Reference") (OtherComp :type "PrimitiveComponent Object Reference") (OtherBodyIndex :type Integer) (bFromSweep :type Boolean) (SweepResult :type "HitResult Structure (by ref)"))
  (`KismetArrayLibrary.Array_Add` (`self.Enemy Array `) OtherActor))

(event `self.ReceiveActorBeginCursorOver`
  (if (`self.Phase 2?`)
    (set `PlayerController.CurrentMouseCursor` "GrabHandClosed" (`GameplayStatics.GetPlayerController` 0))
    (`PrimitiveComponent.SetRenderCustomDepth` (`self.Cube1`) true)
    (`PrimitiveComponent.SetRenderCustomDepth` (`self.Cube`) true)
    (`PrimitiveComponent.SetMaterial` (`self.Cube1`) 0 "/Game/Materials/Mat_master_Black.Mat_master_Black")
    (`PrimitiveComponent.SetMaterial` (`self.Cube`) 0 "/Game/Materials/Mat_master_Black.Mat_master_Black")))

(event `self.ReceiveActorEndCursorOver`
  (if (`self.Phase 2?`)
    (set `PlayerController.CurrentMouseCursor` "GrabHand" (`GameplayStatics.GetPlayerController` 0))
    (`PrimitiveComponent.SetRenderCustomDepth` (`self.Cube1`) false)
    (`PrimitiveComponent.SetRenderCustomDepth` (`self.Cube`) false)
    (`PrimitiveComponent.SetMaterial` (`self.Cube1`) 0 "/Game/Materials/Mat_master_Black_H.Mat_master_Black_H")
    (`PrimitiveComponent.SetMaterial` (`self.Cube`) 0 "/Game/Materials/Mat_master_Black_H.Mat_master_Black_H")))

(event `self.Box.OnComponentEndOverlap`
  (params (OverlappedComponent :type "PrimitiveComponent Object Reference") (OtherActor :type "Actor Object Reference") (OtherComp :type "PrimitiveComponent Object Reference") (OtherBodyIndex :type Integer))
  (if (`KismetArrayLibrary.Array_Contains` (`self.Enemy Array `) OtherActor)
    (`GameplayStatics.ApplyDamage` OtherActor 15.0)
    (`KismetArrayLibrary.Array_RemoveItem` (`self.Enemy Array `) OtherActor)))

(event `/Game/Characters/Player/Game_BPI.Traps go online`
  (`PrimitiveComponent.SetMaterial` (`self.Cube1`) 0 "/Game/Materials/Mat_master_Black_H.Mat_master_Black_H")
  (`PrimitiveComponent.SetMaterial` (`self.Cube`) 0 "/Game/Materials/Mat_master_Black_H.Mat_master_Black_H")
  (set `self.Phase 2?` true))

(fn `UserConstructionScript`)