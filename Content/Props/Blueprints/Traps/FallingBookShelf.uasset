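; Clickable falling bookshelf trap with randomized book meshes, armed when TrapsGoOnline switches it to Phase2.
; Cursor hover swaps the cursor, material and custom-depth outline, and a click plays the ClockFall timeline to tip the shelf over.
; While armed, Box overlaps damage actors other than the player pawn, using the BookShelf row of Traps_DataTable.
; After the fall, the timeline reverses following a short delay to stand the shelf back up.
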(event `self.ReceiveBeginPlay`
  (bind _bookshelf (`self.BookShelf`))
  (`self.Get Random Books `)
  (`PrimitiveComponent.SetMaterial` (`self.BookShelf`) 0 "/Game/Materials/Mat_master_Black.Mat_master_Black")
  (`PrimitiveComponent.SetCollisionResponseToChannel` _bookshelf "ECC_Visibility" "ECR_Block")
  (`PrimitiveComponent.SetCollisionResponseToChannel` _bookshelf "ECC_Pawn" "ECR_Block")
  (`PrimitiveComponent.SetCollisionResponseToChannel` (`self.Box1`) "ECC_Pawn" "ECR_Block"))

(event `Reverse the clock`
  (`|ExecutionSequence`
    (:`then_0`
      (`KismetSystemLibrary.Delay` 3.0)
      (`TimelineComponent.Reverse` (`self.Clock Fall`)))
    (:`then_1`
      (set `self.is Down?` false)
      (set `self.In Progress?` false)
      (`PrimitiveComponent.SetCollisionEnabled` (`self.Box`) "QueryAndPhysics"))))

(event `self.ReceiveActorOnClicked`
  (params (ButtonPressed :type "Key Structure"))
  (if (`self.Phase 2?`) :!label _label
    (if (not (`self.is Down?`))
      (if (not (`self.In Progress?`))
        (`PrimitiveComponent.SetCollisionEnabled` (`self.Box`) "QueryAndPhysics")
        (`TimelineComponent.Stop` (`self.Clock Fall`))
        (set `self.is Down?` true)
        (bind (_direction _fall) (`Timeline|Clock Fall`)
          (:`Update`
            (`SceneComponent.K2_SetRelativeRotation` (`self.BookShelf`) (`KismetMathLibrary.MakeRotator` 0.0 (* _fall -1.0) 90.0) true false)
            (set `self.In Progress?` true))
          (:`Finished`
            (`PrimitiveComponent.SetCollisionEnabled` (`self.Box`) "NoCollision")
            (`self.Reverse the clock`)))))))

(event `self.BookShelf.OnClicked`
  (params (TouchedComponent :type "PrimitiveComponent Object Reference") (ButtonPressed :type "Key Structure"))
  (goto _label))

(event `self.Box1.OnClicked`
  (params (TouchedComponent :type "PrimitiveComponent Object Reference") (ButtonPressed :type "Key Structure"))
  (goto _label))

(event `self.ReceiveActorBeginCursorOver`
  (if (`self.Phase 2?`)
    (set `PlayerController.CurrentMouseCursor` "GrabHandClosed" (`GameplayStatics.GetPlayerController` 0))
    (`PrimitiveComponent.SetRenderCustomDepth` (`self.BookShelf`) true)
    (`PrimitiveComponent.SetMaterial` (`self.BookShelf`) 0 "/Game/Materials/Mat_master_Black.Mat_master_Black")))

(event `self.Box.OnComponentBeginOverlap`
  (params (OverlappedComponent :type "PrimitiveComponent Object Reference") (OtherActor :type "Actor Object Reference") (OtherComp :type "PrimitiveComponent Object Reference") (OtherBodyIndex :type Integer) (bFromSweep :type Boolean) (SweepResult :type "HitResult Structure (by ref)"))
  (if (and (!= OtherActor (`GameplayStatics.GetPlayerPawn` 0)) (`self.Phase 2?`))
    (bind _returnvalue (`|GetDataTableRow` "/Game/Blueprints/Traps_DataTable.Traps_DataTable" "BookShelf")
      (:`then`
        (`GameplayStatics.ApplyDamage` OtherActor (`.Damage_6_666D396E4E7235FFCE84008E808C7946` (break `/Game/Blueprints/TrapsStruct` _returnvalue)) null self)))))

(event `self.ReceiveActorEndCursorOver`
  (if (`self.Phase 2?`)
    (set `PlayerController.CurrentMouseCursor` "GrabHand" (`GameplayStatics.GetPlayerController` 0))
    (`PrimitiveComponent.SetRenderCustomDepth` (`self.BookShelf`) false)
    (`PrimitiveComponent.SetMaterial` (`self.BookShelf`) 0 "/Game/Materials/Mat_master_Black_H.Mat_master_Black_H")))

(event `/Game/Characters/Player/Game_BPI.Traps go online`
  (bind _bookshelf (`self.BookShelf`))
  (`PrimitiveComponent.SetMaterial` (`self.BookShelf`) 0 "/Game/Materials/Mat_master_Black_H.Mat_master_Black_H")
  (`PrimitiveComponent.SetCollisionResponseToChannel` _bookshelf "ECC_Visibility" "ECR_Block")
  (`PrimitiveComponent.SetCollisionResponseToChannel` _bookshelf "ECC_Pawn" "ECR_Ignore")
  (set `self.Phase 2?` true))

(fn `Get Random Books `
  (`StaticMeshComponent.SetStaticMesh` (`self.Books`) (`|GetArrayItem` (`self.Random Books`) (`KismetMathLibrary.RandomIntegerInRange` 0 (`KismetArrayLibrary.Array_Length` (`self.Random Books`))))))

(fn `UserConstructionScript`
  (`self.Get Random Books `))