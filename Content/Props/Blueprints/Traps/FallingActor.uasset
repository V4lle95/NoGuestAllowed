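; FallingActor is a trap prop that drops when clicked and damages actors it overlaps, sparing the player pawn.
; Clicking its Box turns on physics for the static mesh, and a hit turns it off again with query and physics collision enabled.
; If the Destroy flag is set, the actor then waits, spawns an explosion emitter at its location and destroys itself.
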(event `self.Box.OnClicked`
  (params (TouchedComponent :type "PrimitiveComponent Object Reference") (ButtonPressed :type "Key Structure" :default "AnyKey"))
  (`PrimitiveComponent.SetSimulatePhysics` (`self.StaticMesh`) true))

(event `self.ReceiveHit`
  (params (MyComp :type "PrimitiveComponent Object Reference") (Other :type "Actor Object Reference") (OtherComp :type "PrimitiveComponent Object Reference") (bSelfMoved :type Boolean) (HitLocation :type "Vector Structure") (HitNormal :type "Vector Structure") (NormalImpulse :type "Vector Structure") (Hit :type "HitResult Structure (by ref)"))
  (`PrimitiveComponent.SetSimulatePhysics` (`self.StaticMesh`) false)
  (`PrimitiveComponent.SetCollisionEnabled` (`self.StaticMesh`) "QueryAndPhysics")
  (`KismetSystemLibrary.Delay` 0.5)
  (if (`self.Destroy?`)
    (`KismetSystemLibrary.Delay` (`self.Delay Time`))
    (`GameplayStatics.SpawnEmitterAtLocation` "/Game/StarterContent/Particles/P_Explosion.P_Explosion" (`self.K2_GetActorLocation`))
    (`self.K2_DestroyActor`)))

(event `self.StaticMesh.OnComponentBeginOverlap`
  (params (OverlappedComponent :type "PrimitiveComponent Object Reference") (OtherActor :type "Actor Object Reference") (OtherComp :type "PrimitiveComponent Object Reference") (OtherBodyIndex :type Integer) (bFromSweep :type Boolean) (SweepResult :type "HitResult Structure (by ref)"))
  (if (!= OtherActor (`GameplayStatics.GetPlayerPawn` 0))
    (`GameplayStatics.ApplyDamage` OtherActor (`self.Damage`) null self)))

(fn `UserConstructionScript`)