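; Clickable spike trap that slams its spikes down and damages actors caught by them, sparing the player pawn.
; Clicking SpikesCol while SpikeUp is set eases the Spikes component down, pauses briefly, then starts raising it back.
; SpikeUp blocks clicks from the drop until the return begins.
; Any begin overlap on SpikesCol, independent of clicks, applies fixed damage to actors other than player 0's pawn.
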(event `self.SpikesCol.OnClicked`
  (params (TouchedComponent :type "PrimitiveComponent Object Reference") (ButtonPressed :type "Key Structure" :default "AnyKey"))
  (bind _spikes (`self.Spikes`))
  ;[1 1 1] UP/DOWN
  (if (`self.Spike Up?`)
    (set `self.Spike Up?` false)
    (`KismetSystemLibrary.MoveComponentTo` _spikes (0.0 0.0 10.0) (struct) true true 0.5)
    (`KismetSystemLibrary.Delay` 0.6)
    (`KismetSystemLibrary.MoveComponentTo` _spikes (0.0 0.0 640.0) (struct) true true 0.52)
    (set `self.Spike Up?` true)))

(event `self.SpikesCol.OnComponentBeginOverlap`
  (params (OverlappedComponent :type "PrimitiveComponent Object Reference") (OtherActor :type "Actor Object Reference") (OtherComp :type "PrimitiveComponent Object Reference") (OtherBodyIndex :type Integer) (bFromSweep :type Boolean) (SweepResult :type "HitResult Structure (by ref)"))
  ;[1 1 1] Damage
  (if (!= OtherActor (`GameplayStatics.GetPlayerPawn` 0))
    (`GameplayStatics.ApplyDamage` OtherActor 100.0 null self)))

(fn `UserConstructionScript`)