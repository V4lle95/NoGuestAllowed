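; Hammer trap prop that swings a hammer and damages any actor that touches its hit sphere.
; On BeginPlay the RotatedHammer timeline drives the hammer's relative roll from its Alpha track.
; Sphere overlap applies a fixed damage hit to the overlapping actor, with the trap as damage causer.
; An older MoveComponentTo-and-Delay swing sequence remains in the graph but is disconnected.
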(event `self.ReceiveTick`
  (params (DeltaSeconds :type "Float (single-precision)")))

(event `self.Sphere.OnComponentBeginOverlap`
  (params (OverlappedComponent :type "PrimitiveComponent Object Reference") (OtherActor :type "Actor Object Reference") (OtherComp :type "PrimitiveComponent Object Reference") (OtherBodyIndex :type Integer) (bFromSweep :type Boolean) (SweepResult :type "HitResult Structure (by ref)"))
  (`GameplayStatics.ApplyDamage` OtherActor 100.0 null self))

(event `self.ReceiveBeginPlay`
  (bind (_direction _alpha) (`Timeline|Rotated Hammer` :!via `PlayFromStart`)
    (:`Update`
      (`SceneComponent.K2_SetRelativeRotation` (`self.Hammer`) (`KismetMathLibrary.MakeRotator` _alpha) false false))))

(fn `UserConstructionScript`)