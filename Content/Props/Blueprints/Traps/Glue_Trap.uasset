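; Glue trap prop that, once TrapsGoOnline enables Phase2, can be clicked on and off to slow AI_Guard actors inside its box.
; Clicks flip the box's Pawn response between Overlap and Ignore, while a timeline drives the Glue material parameter collection.
; Hovering changes cursor, outline and material.
; BeginPlay disables box collision, never re-enabled here, and reads the restore speed by casting the player pawn to AI_Guard.
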(event `self.Box.OnComponentBeginOverlap`
  (params (OverlappedComponent :type "PrimitiveComponent Object Reference") (OtherActor :type "Actor Object Reference") (OtherComp :type "PrimitiveComponent Object Reference") (OtherBodyIndex :type Integer) (bFromSweep :type Boolean) (SweepResult :type "HitResult Structure (by ref)"))
  (bind _asai_guard (cast `/Game/Characters/Ai/Enemy/AI_Guard` OtherActor))
  (set `CharacterMovementComponent.MaxWalkSpeed` (`self.Slow Walk Speed`) (`Character.CharacterMovement` _asai_guard)))

(event `self.Box.OnComponentEndOverlap`
  (params (OverlappedComponent :type "PrimitiveComponent Object Reference") (OtherActor :type "Actor Object Reference") (OtherComp :type "PrimitiveComponent Object Reference") (OtherBodyIndex :type Integer))
  (bind _asai_guard (cast `/Game/Characters/Ai/Enemy/AI_Guard` OtherActor))
  (set `CharacterMovementComponent.MaxWalkSpeed` (`self.Regular Speed`) (`Character.CharacterMovement` _asai_guard)))

(event `self.Cube.OnClicked`
  (params (TouchedComponent :type "PrimitiveComponent Object Reference") (ButtonPressed :type "Key Structure"))
  (bind _box (`self.Box`))
  (if (`self.Phase 2?`)
    (`/Engine/EditorBlueprintResources/StandardMacros.FlipFlop`
      (:`A`
        (`PrimitiveComponent.SetCollisionResponseToChannel` _box "ECC_Pawn" "ECR_Overlap")
        (bind (_direction _alpha) (`Timeline|Glue TT` :!via `PlayFromStart`)
          (:`Update`
            (`KismetMaterialLibrary.SetScalarParameterValue` "/Game/Materials/Decal/Glue.Glue" "Value" _alpha))))
      (:`B`
        (`PrimitiveComponent.SetCollisionResponseToChannel` _box "ECC_Pawn" "ECR_Ignore")
        (`TimelineComponent.ReverseFromEnd` (`self.Glue TT`))))))

(event `self.ReceiveActorBeginCursorOver`
  (if (`self.Phase 2?`)
    (set `PlayerController.CurrentMouseCursor` "GrabHandClosed" (`GameplayStatics.GetPlayerController` 0))
    (`PrimitiveComponent.SetRenderCustomDepth` (`self.Cube`) true)
    (`PrimitiveComponent.SetMaterial` (`self.Cube`) 0 "/Game/Materials/Mat_master_Concrete.Mat_master_Concrete")))

(event `self.ReceiveActorEndCursorOver`
  (if (`self.Phase 2?`)
    (set `PlayerController.CurrentMouseCursor` "GrabHand" (`GameplayStatics.GetPlayerController` 0))
    (`PrimitiveComponent.SetRenderCustomDepth` (`self.Cube`) false)
    (`PrimitiveComponent.SetMaterial` (`self.Cube`) 0 "/Game/Materials/Mat_master_Concrete_H.Mat_master_Concrete_H")))

(event `self.ReceiveBeginPlay`
  (`PrimitiveComponent.SetMaterial` (`self.Cube`) 0 "/Game/Materials/Mat_master_Concrete.Mat_master_Concrete")
  (bind _asai_guard (cast `/Game/Characters/Ai/Enemy/AI_Guard` (`GameplayStatics.GetPlayerPawn` 0)))
  (set `self.Regular Speed` (`CharacterMovementComponent.MaxWalkSpeed` (`Character.CharacterMovement` _asai_guard)))
  (`PrimitiveComponent.SetCollisionEnabled` (`self.Box`) "NoCollision")
  (`KismetMaterialLibrary.SetScalarParameterValue` "/Game/Materials/Decal/Glue.Glue" "Value"))

(event `/Game/Characters/Player/Game_BPI.Traps go online`
  (`PrimitiveComponent.SetMaterial` (`self.Cube`) 0 "/Game/Materials/Mat_master_Concrete_H.Mat_master_Concrete_H")
  (set `self.Phase 2?` true))

(fn `UserConstructionScript`)