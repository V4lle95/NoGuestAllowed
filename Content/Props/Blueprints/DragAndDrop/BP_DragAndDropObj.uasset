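; Draggable puzzle prop that snaps onto a nearby BP_TargetObject with a matching ID.
; While active, Tick runs attach checking and cursor-trace dragging on X/Z, though the grab condition includes a literal false and never attaches.
; When unattached, it simulates physics and sphere-traces for the closest target; a match snaps, triggers the target, spawns smoke and destroys both.
; Hovering shows a hand cursor and custom-depth highlight.
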(event `self.ReceiveBeginPlay`
  ;[1 1 1] Player Ref
  (bind _asghost_soul_camera (cast `/Game/Characters/Player/Phase_2/Ghost_Soul_Camera` (`Controller.K2_GetPawn` (`GameplayStatics.GetPlayerController` 0))))
  (set `self.Player` _asghost_soul_camera))

(event `self.ReceiveActorOnClicked`
  (params (ButtonPressed :type "Key Structure" :default "AnyKey")))

(event `self.ReceiveActorOnInputTouchBegin`
  (params (FingerIndex :type "ETouchIndex Enum" :default "Touch1")))

(event `self.ReceiveActorOnReleased`
  (params (ButtonReleased :type "Key Structure" :default "AnyKey")))

(event `self.ReceiveActorOnInputTouchEnd`
  (params (FingerIndex :type "ETouchIndex Enum" :default "Touch1")))

(event `self.ReceiveActorBeginCursorOver`
  (set `PlayerController.CurrentMouseCursor` "Hand" (`GameplayStatics.GetPlayerController` 0))
  (set `self.Cursor Hover` true)
  (`PrimitiveComponent.SetRenderCustomDepth` (`self.StaticMesh`) true))

(event `self.ReceiveActorEndCursorOver`
  (set `PlayerController.CurrentMouseCursor` "Default" (`GameplayStatics.GetPlayerController` 0))
  (set `self.Cursor Hover` false)
  (`PrimitiveComponent.SetRenderCustomDepth` (`self.StaticMesh`) false))

(event `Check attach`
  (`/Engine/EditorBlueprintResources/StandardMacros.IsValid` null
    (:`Is Valid`
      (if (and (`self.Cursor Hover`) false)
        (`self.Get attach` true)
        (else
          (`self.Get attach` false)
          (`self.Cheack Target`))))))

(event `Destroy Actors`
  (bind _target_object (`self.Target Object`))
  (`/Game/Props/Blueprints/DragAndDrop/BP_TargetObject.Do Somethin?` _target_object)
  (`KismetSystemLibrary.Delay` 0.5)
  (`GameplayStatics.SpawnEmitterAtLocation` "/Game/Materials/FX/Smoke_FX.Smoke_FX" (`self.K2_GetActorLocation`))
  (`KismetSystemLibrary.Delay` 0.5)
  (`self.K2_DestroyActor` _target_object)
  (`self.K2_DestroyActor`))

(event `Pickup Mesh`
  (bind (_returnvalue_x _returnvalue_y) (`KismetMathLibrary.BreakVector` (`self.K2_GetActorLocation`)))
  (bind (_worldlocation _worlddirection _returnvalue) (`PlayerController.DeprojectMousePositionToWorld` (`GameplayStatics.GetPlayerController` 0)))
  (if _returnvalue
    (if (`self.attach to cursor`)
      (bind (_outhit _returnvalue_2) (`KismetSystemLibrary.LineTraceSingle` _worldlocation (+ _worldlocation (* _worlddirection 10000.0)) "TraceTypeQuery3" false (`|MakeArray` self :!type "Actor Object Reference")))
      (if _returnvalue_2
        (`self.K2_SetActorLocation` (`KismetMathLibrary.MakeVector` (.x (+ (`.Location` (`GameplayStatics.BreakHitResult` _outhit)) (0.0 100.0 0.0))) _returnvalue_y (.z (+ (`.Location` (`GameplayStatics.BreakHitResult` _outhit)) (0.0 100.0 0.0)))) true)))))

(event `self.ReceiveTick`
  (params (DeltaSeconds :type "Float (single-precision)"))
  (if (`self.Is Active`)
    (`self.Check attach`)
    (`self.Pickup Mesh`)))

(event `self.StaticMesh.OnComponentHit`
  (params (HitComponent :type "PrimitiveComponent Object Reference") (OtherActor :type "Actor Object Reference") (OtherComp :type "PrimitiveComponent Object Reference") (NormalImpulse :type "Vector Structure") (Hit :type "HitResult Structure (by ref)"))
  (`PrimitiveComponent.SetSimulatePhysics` (`self.StaticMesh`) false))

(fn `Cheack Target`
  (bind _staticmesh (`self.StaticMesh`))
  (bind _target_object (`self.Target Object`))
  (bind _returnvalue (`SceneComponent.K2_GetComponentLocation` (`self.StaticMesh`)))
  (bind (_outhits _returnvalue_2) (`KismetSystemLibrary.SphereTraceMulti` :`Start` _returnvalue :`End` (+ _returnvalue (0.0 2.0 0.0)) :`Radius` 200.0 :`TraceChannel` "TraceTypeQuery1" :`DrawDebugType` "ForOneFrame"))
  (if _returnvalue_2
    (for (_array_element _array_index) _outhits
      (bind (_bblockinghit _binitialoverlap _time _location _impactpoint _normal _impactnormal _physmat _hitactor _hitcomponent _hitbonename _hititem _faceindex _tracestart) (`GameplayStatics.BreakHitResult` _array_element))
      (bind _asbp_target_object (cast `/Game/Props/Blueprints/DragAndDrop/BP_TargetObject` _hitactor))
      (if (== _array_index 0)
        (set `self.Target Object` _asbp_target_object)
        (bind _returnvalue_3 (`KismetMathLibrary.VSize` (- (`SceneComponent.K2_GetComponentLocation` (`/Game/Props/Blueprints/DragAndDrop/BP_TargetObject.StaticMesh` _asbp_target_object)) _tracestart)))
        (set `self.Target Distance` _returnvalue_3)
        (elif (< _returnvalue_3 (`self.Target Distance`))
          (set `self.Target Object` _asbp_target_object)
          (set `self.Target Distance` _returnvalue_3))))
    (`/Engine/EditorBlueprintResources/StandardMacros.IsValid` _target_object
      (:`Is Valid`
        (if (<= (`self.Target Distance`) (`self.MinTargetDistance`))
          (if (== (`/Game/Props/Blueprints/DragAndDrop/BP_TargetObject.ID` _target_object) (`self.ID`))
            (`PrimitiveComponent.SetSimulatePhysics` _staticmesh false)
            (set `self.Is Active` false)
            (`SceneComponent.K2_SetWorldLocation` _staticmesh (`SceneComponent.K2_GetComponentLocation` (`/Game/Props/Blueprints/DragAndDrop/BP_TargetObject.StaticMesh` (`self.Target Object`))) false false)
            (`self.Destroy Actors`)))))))

(fn `Get attach`
  (params (Attachted :type Boolean))
  (`PrimitiveComponent.SetSimulatePhysics` (`self.StaticMesh`) (not Attachted))
  (set `self.attach to cursor` Attachted))

(fn `UserConstructionScript`)